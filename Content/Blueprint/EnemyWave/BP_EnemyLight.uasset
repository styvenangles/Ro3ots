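; BP_EnemyLight is an enemy, from the EnemyWave folder, that chases the player and can damage them.
; One second after BeginPlay it targets the player's pawn, then Tick drives a delayed AIMoveTo until flagged as in range.
; InRangeEnemy sets that flag from the "Player" tag, and AttackEnemy applies AttackDamage to BP_ThirdPersonCharacter, matched by class display name.
; Neither event is called within this graph.
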(event Custom|MoveToPlayer
  (params (Enemy :type Actor%20Object%20Reference) (EnemyLocation :type Vector))
  (Utilities|FlowControl|Delay 0.5)
  (AI|AIMoveTo self EnemyLocation Enemy 5.0 false))

(event EventBeginPlay
  (bind _returnvalue (Game|GetPlayerController 0))
  (bind _returnvalue_2 (Pawn|GetControlledPawn _returnvalue))
  (Utilities|FlowControl|Delay 1.0)
  (if (!= _returnvalue 0)
    (Class|AttackSystem|TargetEnemy _returnvalue_2 (Transformation|GetActorLocation _returnvalue_2) false)))

(event Collision|EventActorBeginOverlap
  (params (OtherActor :type Actor%20Object%20Reference)))

(event EventTick
  (params (DeltaSeconds :type Float%20%28single-precision%29))
  (bind _targetactor (Variables|Default|GettargetActor))
  (if (!= _targetactor 0)
    (if (not (Variables|Default|GetisInRangeToAttack))
      (CallFunction|MovetoPlayer _targetactor (Variables|Default|GetEnemy%20Location)))))

(event EventTargetEnemy
  (params (Enemy :type Actor%20Object%20Reference) (Location :type Vector :default "0, 0, 0") (isPlayer :type Boolean))
  (Variables|Default|SettargetActor Enemy)
  (Variables|Default|SetEnemy%20Location Location))

(event EventInRangeEnemy
  (params (Enemy :type Actor%20Object%20Reference) (isPlayer :type Boolean))
  (if (Actor|ActorHasTag Enemy "Player")
    (Variables|Default|SetisInRangeToAttack true)
    (else
      (Variables|Default|SetisInRangeToAttack false))))

(event EventAttackEnemy
  (params (Enemy :type Actor%20Object%20Reference) (Damage :type Float%20%28single-precision%29) (isPlayer :type Boolean))
  (if (!= Enemy 0)
    (switch string (Utilities|GetClassDisplayName (Utilities|GetClass Enemy))
      (:BP_ThirdPersonCharacter_C
        (bind _asbp_third_person_character (Utilities|Casting|CastToBP_ThirdPersonCharacter Enemy))
        (Class|Ro3otsCharacter|TakeDamage _asbp_third_person_character (Math|Float|Truncate (Variables|Default|GetAttackDamage)))))))

(fn ConstructionScript)